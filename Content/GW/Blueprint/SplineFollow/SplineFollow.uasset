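; Spline path actor that steers every CarCubeAIBP vehicle along its Path spline, updated each Tick.
; It projects a point offset along the path direction from each car onto the spline and writes it to Steering as a look-ahead target.
; AutoThrottle eases off as forward speed times horizontal distance from the spline grows, via an unclamped remap.
; Sphere marks the target; Arrow marks the closest point and feeds that distance check.
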(event `self.ReceiveTick`
  (params (DeltaSeconds :type "Float (single-precision)"))
  (bind (_returnvalue_roll _returnvalue_pitch _returnvalue_yaw) (`KismetMathLibrary.BreakRotator` (`self.K2_GetActorRotation`)))
  (bind _path (`self.Path`))
  (bind (_returnvalue_x _returnvalue_y) (`KismetMathLibrary.BreakVector` (`SceneComponent.K2_GetComponentLocation` (`self.Arrow`))))
  (bind _outactors (`GameplayStatics.GetAllActorsOfClass` "/Game/GW/Blueprint/SplineFollow/CarCubeAIBP.CarCubeAIBP_C"))
  (for _array_element _outactors
    (bind _returnvalue (`self.K2_GetActorLocation` _array_element))
    (bind _returnvalue_2 (`KismetMathLibrary.MakeRotationFromAxes` (`KismetMathLibrary.GreaterGreater_VectorRotator` (`SplineComponent.FindRightVectorClosestToWorldLocation` _path _returnvalue "Local") (`KismetMathLibrary.MakeRotator` _returnvalue_roll _returnvalue_pitch (+ _returnvalue_yaw 90.0)))))
    (bind _output_get (set `/Game/GW/Blueprint/SplineFollow/CarCubeAIBP.Steering` (`SplineComponent.FindLocationClosestToWorldLocation` _path (- _returnvalue (* (`KismetMathLibrary.GetForwardVector` _returnvalue_2) 500)) "World") _array_element))
    (`SceneComponent.K2_SetWorldLocation` (`self.Sphere`) _output_get false false)
    (`SceneComponent.K2_SetWorldLocationAndRotation` (`self.Arrow`) (`SplineComponent.FindLocationClosestToWorldLocation` _path _returnvalue "World") (`KismetMathLibrary.MakeRotator` (.roll _returnvalue_2) (.pitch _returnvalue_2) (- (.yaw _returnvalue_2) 180.0)) false false)
    (bind _returnvalue_3 (* (`WheeledVehicleMovementComponent.GetForwardSpeed` (`WheeledVehicle.VehicleMovement` _array_element)) 0.36))
    (bind (_returnvalue_x_2 _returnvalue_y_2) (`KismetMathLibrary.BreakVector` (`self.K2_GetActorLocation` _array_element)))
    (bind _returnvalue_4 (* _returnvalue_3 (`KismetMathLibrary.VSize` (- (`KismetMathLibrary.MakeVector` _returnvalue_x_2 _returnvalue_y_2) (`KismetMathLibrary.MakeVector` _returnvalue_x _returnvalue_y)))))
    (bind _output_get_2 (set `/Game/GW/Blueprint/SplineFollow/CarCubeAIBP.AutoThrottle` (`KismetMathLibrary.SelectFloat` 1.0 (`KismetMathLibrary.SelectFloat` 1.0 (`KismetMathLibrary.MapRangeUnclamped` _returnvalue_4 0.0 10000.0 1.0 0.9) (< _returnvalue_4 1000.0)) (< _returnvalue_3 0.0)) _array_element))))

(fn `UserConstructionScript`)