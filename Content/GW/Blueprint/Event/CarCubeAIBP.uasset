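; AI-driven cube car for a race, steered by SteeringCalc (its look-at math is unused) with automatic throttle while the race runs.
; It registers its start transform with MyPlayerController by AINumber.
; If it stays flipped and slow across a four-second delay, it destroys itself and the controller respawns it.
; Box overlaps reduce a CarCubeBP's HealNum, and Brake input toggles the handbrake.
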(event `self.ReceiveBeginPlay`
  ;[1 1 1] Begin
  (`KismetSystemLibrary.ExecuteConsoleCommand` "show splines" null)
  (bind _asmy_player_controller (cast `/Game/GW/Blueprint/Event/MyPlayerController` (`GameplayStatics.GetPlayerController` 0)))
  (bind _output_get (set `self.ControllerReff` _asmy_player_controller))
  (`KismetArrayLibrary.Array_Set` (`/Game/GW/Blueprint/Event/MyPlayerController.RespawnLocationAI` _output_get) (`self.AINumber`) (`self.GetTransform`)))

(event `self.ReceiveTick`
  (params (DeltaSeconds :type "Float (single-precision)"))
  (bind _vehiclemovement (`self.VehicleMovement`))
  (bind _controllerreff (`self.ControllerReff`))
  ;[1 1 1] Basic Controller
  (if (`/Game/GW/Blueprint/Event/MyPlayerController.RaceComplete` _controllerreff)
    _
    (elif (`/Game/GW/Blueprint/Event/MyPlayerController.RaceStart` _controllerreff)
      (`WheeledVehicleMovementComponent.SetSteeringInput` _vehiclemovement (`self.SteeringCalc`))
      (`WheeledVehicleMovementComponent.SetThrottleInput` _vehiclemovement (`self.AutoThrottle`))
      (bind _playerisstuck (`self.RespawnCheck`))
      (if _playerisstuck
        (`KismetSystemLibrary.Delay` 4.0)
        (bind _playerisstuck_2 (`self.RespawnCheck`))
        (if _playerisstuck_2
          (`self.K2_DestroyActor`))))))

(event `self.ReceiveDestroyed`
  ;[1 1 1] Basic Controller
  (`/Game/GW/Blueprint/Event/MyPlayerController.RespawnVehicleAI` (`self.ControllerReff`) (`self.AINumber`)))

(event `InputAction|Brake`
  (params (Key :type "Key Structure"))
  (bind _vehiclemovement (`self.VehicleMovement`))
  ;[1 1 1] Basic Controller
  (:`Pressed`
    (`WheeledVehicleMovementComponent.SetHandbrakeInput` _vehiclemovement true))
  (:`Released`
    (`WheeledVehicleMovementComponent.SetHandbrakeInput` _vehiclemovement false)))

(event `self.Box.OnComponentBeginOverlap`
  (params (OverlappedComponent :type "PrimitiveComponent Object Reference") (OtherActor :type "Actor Object Reference") (OtherComp :type "PrimitiveComponent Object Reference") (OtherBodyIndex :type Integer) (bFromSweep :type Boolean) (SweepResult :type "HitResult Structure (by ref)"))
  ;[1 1 1] Overlap CarCubeBP
  (bind _ascar_cube_bp (cast `/Game/GW/Blueprint/Player/CarCubeBP` OtherActor))
  (set `/Game/GW/Blueprint/Player/CarCubeBP.Heal_Num` (- (`/Game/GW/Blueprint/Player/CarCubeBP.Heal_Num` _ascar_cube_bp) 0.1) _ascar_cube_bp))

(fn `RespawnCheck`
  (returns (PlayerIsStuck :type Boolean))
  ;[1 1 1] Check and See if the player is not moving is upsidedown
  (if (and (< (`KismetMathLibrary.Dot_VectorVector` (`self.GetActorUpVector`) (0.0 0.0 1.0)) 0.5) (< (`WheeledVehicleMovementComponent.GetForwardSpeed` (`self.VehicleMovement`)) 0.5))
    (set `self.Stuck` true)
    (else
      (set `self.Stuck` false)))
  (return (`self.Stuck`)))

(fn `UserConstructionScript`)