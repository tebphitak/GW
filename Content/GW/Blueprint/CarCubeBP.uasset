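; Player-driven race car that maps axis and brake input to throttle, steering and handbrake on its vehicle movement component.
; Input stays disabled until the player controller flags race start; BeginPlay also stores the spawn transform there as the respawn location.
; Tick detects a tipped, slow car, rechecks after a delay, then destroys it, and Destroyed asks the controller to respawn it.
; Overlapping pickups increase two bullet counters and a heal counter.
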(event `self.ReceiveBeginPlay`
  ;[1 1 1] Begin
  (bind _asmy_player_controller (cast `/Game/GW/Blueprint/Event/MyPlayerController` (`GameplayStatics.GetPlayerController` 0)))
  (bind _output_get (set `self.ControllerReff` _asmy_player_controller))
  (set `/Game/GW/Blueprint/Event/MyPlayerController.RespawnLocation` (`self.GetTransform`) _output_get)
  (`self.DisableInput` (`self.ControllerReff`)))

(event `self.ReceiveTick`
  (params (DeltaSeconds :type "Float (single-precision)"))
  (bind _controllerreff (`self.ControllerReff`))
  ;[1 1 1] Checking if player has flipped their car and is stuck, if so, call Respawn vehicle in MyPlayerController
  (if (`/Game/GW/Blueprint/Event/MyPlayerController.RaceStart` _controllerreff)
    (`self.EnableInput` _controllerreff)
    (bind _playerisstuck (`self.RespawnCheck`))
    (if _playerisstuck
      (`KismetSystemLibrary.Delay` 4.0)
      (bind _playerisstuck_2 (`self.RespawnCheck`))
      (if _playerisstuck_2
        (`self.K2_DestroyActor`)))))

(event `self.ReceiveDestroyed`
  ;[1 1 1] Checking if player has flipped their car and is stuck, if so, call Respawn vehicle in MyPlayerController
  (`/Game/GW/Blueprint/Event/MyPlayerController.RespawnVehicle` (`self.ControllerReff`)))

(event `InputAxis|Forward`
  (params (AxisValue :type "Float (single-precision)"))
  ;[1 1 1] Basic Controller
  (`WheeledVehicleMovementComponent.SetThrottleInput` (`self.VehicleMovement`) AxisValue))

(event `InputAxis|Right`
  (params (AxisValue :type "Float (single-precision)"))
  ;[1 1 1] Basic Controller
  (`WheeledVehicleMovementComponent.SetSteeringInput` (`self.VehicleMovement`) AxisValue))

(event `InputAction|Brake`
  (params (Key :type "Key Structure"))
  (bind _vehiclemovement (`self.VehicleMovement`))
  ;[1 1 1] Basic Controller
  (:`Pressed`
    (`WheeledVehicleMovementComponent.SetHandbrakeInput` _vehiclemovement true))
  (:`Released`
    (`WheeledVehicleMovementComponent.SetHandbrakeInput` _vehiclemovement false)))

(event `self.ReceiveActorBeginOverlap`
  (params (OtherActor :type "Actor Object Reference"))
  ;[1 1 1] Collect BBullet
  (cast `/Game/GW/Item/Bullet/BBullet_Obj/BBullet_Obj` OtherActor
    (:`then`
      (set `self.BBullet_Num` (+ (`self.BBullet_Num`) 5)))
    (:`CastFailed`
      (cast `/Game/GW/Item/Bullet/SBullet_Obj/SBullet_Obj` OtherActor
        (:`then`
          (set `self.SBullet_Num` (+ (`self.SBullet_Num`) 5)))
        (:`CastFailed`
          (cast `/Game/GW/Item/Heal/Heal/Heal_Obj/Heal_Obj` OtherActor)
          (set `self.Heal_Num` (+ (`self.Heal_Num`) 1.0)))))))

(fn `RespawnCheck`
  (returns (PlayerIsStuck :type Boolean))
  ;[1 1 1] Check and See if the player is not moving is upsidedown
  (if (and (< (`KismetMathLibrary.Dot_VectorVector` (`self.GetActorUpVector`) (0.0 0.0 1.0)) 0.5) (< (`WheeledVehicleMovementComponent.GetForwardSpeed` (`self.VehicleMovement`)) 0.5))
    (set `self.Stuck` true)
    (else
      (set `self.Stuck` false)))
  (return (`self.Stuck`)))

(fn `UserConstructionScript`)