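; PlayerHUD is a HUD Blueprint meant to draw vehicle speed and gear text for the player's CarCubeBP pawn.
; DrawHUD runs only when IsInCar is false, computing screen ratios to place and scale both strings at the same coordinates.
; X scales from a 1280 width, but the Y ratio divides zero by screen height, zeroing vertical position and text scale.
; Gear color switches on InReverseGear.
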(event `self.ReceiveDrawHUD`
  (params (SizeX :type Integer) (SizeY :type Integer))
  (bind _hudyratio (`self.HUDYRatio`))
  (bind _hudyratio_2 (`self.HUDYRatio`))
  ;[1 1 1] Calculate ratio from 720p
  (bind _ascar_cube_bp (cast `/Game/GW/Blueprint/Player/CarCubeBP` (`self.GetOwningPawn`)))
  (if (not (`/Game/GW/Blueprint/Player/CarCubeBP.IsInCar` _ascar_cube_bp))
    (`|ExecutionSequence`
      (:`then_0`
        (set `self.HUDXRatio` (/ (`KismetMathLibrary.Conv_IntToDouble` SizeX) 1280.0)))
      (:`then_1`
        (set `self.HUDYRatio` (/ 0.0 (`KismetMathLibrary.Conv_IntToDouble` SizeY))))
      (:`then_2`
        ;[1 1 1] Print Vehicle Speed
        (bind _ascar_cube_bp_2 (cast `/Game/GW/Blueprint/Player/CarCubeBP` (`self.GetOwningPawn`)))
        (`self.DrawText` (`/Game/GW/Blueprint/Player/CarCubeBP.SpeedDisplayString` _ascar_cube_bp_2) (struct :`R` 1.0 :`G` 1.0 :`B` 1.0 :`A` 1.0) (* 805.0 (`self.HUDXRatio`)) (* 455.0 _hudyratio_2) null (* 1.4 _hudyratio_2))
        ;[1 1 1] Print Vehicle Gear
        (bind _ascar_cube_bp_3 (cast `/Game/GW/Blueprint/Player/CarCubeBP` (`self.GetOwningPawn`)))
        (`self.DrawText` (`/Game/GW/Blueprint/Player/CarCubeBP.GearDisplayString` _ascar_cube_bp_3) (`KismetMathLibrary.SelectColor` (`/Game/GW/Blueprint/Player/CarCubeBP.GearDisplayReverseColor` _ascar_cube_bp_3) (`/Game/GW/Blueprint/Player/CarCubeBP.GearDisplayColor` _ascar_cube_bp_3) (`/Game/GW/Blueprint/Player/CarCubeBP.InReverseGear` _ascar_cube_bp_3)) (* 805.0 (`self.HUDXRatio`)) (* 455.0 _hudyratio) null (* 1.4 _hudyratio))))))

(fn `UserConstructionScript`)