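; AI vehicle Blueprint intended to follow a spline path in the world.
; On BeginPlay it stores the first SplineBP actor found as its track.
; A Track timeline update would set its location along that spline at a distance derived from game time and Speed, without changing rotation.
; Nothing starts that timeline, so the movement logic never runs.
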(event `self.ReceiveBeginPlay`
  ;[1 1 1] Vehicle Spline Path Follow
  (`|ExecutionSequence`
    (:`then_0`
      (bind _outactors (`GameplayStatics.GetAllActorsOfClass` "/Game/GW/Blueprint/AI/SplineBP.SplineBP_C"))
      (set `self.Spline Track` (`|GetArrayItem` _outactors)))))

(fn `UserConstructionScript`)