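; AI-named battle mode car Blueprint with front and rear health widgets that is removed from play once dead.
; BeginPlay casts both widgets to AIHP and sets the car as their owner.
; Tick polls IsDead and destroys the actor when it is true.
; Basic throttle, steering and handbrake input bindings drive the vehicle movement component; the graph itself holds no AI decision logic.
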(event `self.ReceiveBeginPlay`
  (bind _asaihp (cast `/Game/GW/Blueprint/BattleMode/AIHP` (`WidgetComponent.GetUserWidgetObject` (`self.WidgetHPFront`))))
  (set `/Game/GW/Blueprint/BattleMode/AIHP.Owner` self _asaihp)
  (bind _asaihp_2 (cast `/Game/GW/Blueprint/BattleMode/AIHP` (`WidgetComponent.GetUserWidgetObject` (`self.WidgetHPBack`))))
  (set `/Game/GW/Blueprint/BattleMode/AIHP.Owner` self _asaihp_2))

(event `self.ReceiveTick`
  (params (DeltaSeconds :type "Float (single-precision)"))
  (if (`self.IsDead`)
    (`self.K2_DestroyActor`)))

(event `InputAxis|Forward`
  (params (AxisValue :type "Float (single-precision)"))
  ;[1 1 1] Basic Controller
  (`WheeledVehicleMovementComponent.SetThrottleInput` (`self.VehicleMovement`) AxisValue))

(event `InputAxis|Right`
  (params (AxisValue :type "Float (single-precision)"))
  ;[1 1 1] Basic Controller
  (`WheeledVehicleMovementComponent.SetSteeringInput` (`self.VehicleMovement`) AxisValue))

(event `InputAction|Brake`
  (params (Key :type "Key Structure"))
  (bind _vehiclemovement (`self.VehicleMovement`))
  ;[1 1 1] Basic Controller
  (:`Pressed`
    (`WheeledVehicleMovementComponent.SetHandbrakeInput` _vehiclemovement true))
  (:`Released`
    (`WheeledVehicleMovementComponent.SetHandbrakeInput` _vehiclemovement false)))

(fn `UserConstructionScript`)