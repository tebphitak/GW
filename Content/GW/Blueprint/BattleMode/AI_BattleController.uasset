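; AI controller for the AI-driven battle car in battle mode, an unfinished patrol-and-hunt behavior.
; On BeginPlay it copies the waypoint list from its BattleCarAIBP pawn, starts a looping CheckEnemy timer and sends the pawn to the current waypoint.
; CheckEnemy, Patroling and OnHunt are empty stubs, and disconnected move and delayed-patrol nodes never run, so no further waypoint move follows the first.
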(event `self.ReceiveBeginPlay`
  (bind _asbattle_car_aibp (cast `/Game/GW/Blueprint/BattleMode/BattleCarAIBP` (`self.K2_GetPawn`)))
  (set `self.WayPoints` (`/Game/GW/Blueprint/BattleMode/BattleCarAIBP.WayPoint` _asbattle_car_aibp))
  (bind _returnvalue (`KismetSystemLibrary.K2_SetTimer` null "CheckEnemy" 0.3 true))
  (set `self.CleanTimer` _returnvalue)
  (`|AIMoveTo` _asbattle_car_aibp (0.0 0.0 0.0) (`|GetArrayItem` (`self.WayPoints`) (`self.CurrentWayPoint`))))

(event `Patroling`)

(event `OnHunt`)

(event `CheckEnemy`)

(fn `UserConstructionScript`)